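; Elevator actor with proximity-driven sliding panels and an interact-triggered moving platform.
; Overlapping Box plays a timeline that slides Cube5 and Cube6 apart; leaving reverses it.
; Box1 creates and shows a WB_ESign widget on each overlap, then hides it on exit.
; Interact plays a second timeline moving Cube4 along a spline, with no reverse path.
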(event OnComponentBeginOverlap(Box)
  (params (OverlappedComponent :type Primitive%20Component%20Object%20Reference) (OtherActor :type Actor%20Object%20Reference) (OtherComp :type Primitive%20Component%20Object%20Reference) (OtherBodyIndex :type Integer) (bFromSweep :type Boolean) (SweepResult :type Hit%20Result%20Structure%20%28by%20ref%29))
  (bind _newtrack_0 (Timeline|Timeline Play)
    (:Update
      (Transformation|SetRelativeLocation (Variables|Default|GetCube5) (Math|Vector|MakeVector (Math|Float|Lerp -28.0 -74.0 _newtrack_0) 51.0 -8e+02) false false)
      (Transformation|SetRelativeLocation (Variables|Default|GetCube6) (Math|Vector|MakeVector (Math|Float|Lerp 28.0 74.0 _newtrack_0) 51.0 -8e+02) false false))))

(event OnComponentEndOverlap(Box)
  (params (OverlappedComponent :type Primitive%20Component%20Object%20Reference) (OtherActor :type Actor%20Object%20Reference) (OtherComp :type Primitive%20Component%20Object%20Reference) (OtherBodyIndex :type Integer))
  (bind _newtrack_0 (Timeline|Timeline Reverse)
    (:Update
      (Transformation|SetRelativeLocation (Variables|Default|GetCube5) (Math|Vector|MakeVector (Math|Float|Lerp -28.0 -74.0 _newtrack_0) 51.0 -8e+02) false false)
      (Transformation|SetRelativeLocation (Variables|Default|GetCube6) (Math|Vector|MakeVector (Math|Float|Lerp 28.0 74.0 _newtrack_0) 51.0 -8e+02) false false))))

(event OnComponentBeginOverlap(Box1)
  (params (OverlappedComponent :type Primitive%20Component%20Object%20Reference) (OtherActor :type Actor%20Object%20Reference) (OtherComp :type Primitive%20Component%20Object%20Reference) (OtherBodyIndex :type Integer) (bFromSweep :type Boolean) (SweepResult :type Hit%20Result%20Structure%20%28by%20ref%29))
  (bind _returnvalue (UserInterface|CreateWidget "/Game/Custom/Widgets/WB_ESign.WB_ESign_C"))
  (bind _output_get (Variables|Default|SetESignWidget _returnvalue))
  (UserInterface|Viewport|AddtoViewport _output_get 0)
  (Widget|SetVisibility _output_get "Visible"))

(event OnComponentEndOverlap(Box1)
  (params (OverlappedComponent :type Primitive%20Component%20Object%20Reference) (OtherActor :type Actor%20Object%20Reference) (OtherComp :type Primitive%20Component%20Object%20Reference) (OtherBodyIndex :type Integer))
  (bind _output_get (Variables|Default|SetESignWidget (Variables|Default|GetESignWidget)))
  (Widget|SetVisibility _output_get "Hidden"))

(event EventBeginPlay)

(event Collision|EventActorBeginOverlap
  (params (OtherActor :type Actor%20Object%20Reference)))

(event EventTick
  (params (DeltaSeconds :type Float%20%28single-precision%29)))

(event EventInteract
  (bind _newtrack_0 (Timeline|Timeline_0 Play)
    (:Update
      (Transformation|SetWorldLocation (Variables|Default|GetCube4) (Spline|GetLocationatTime (Variables|Default|GetSpline) _newtrack_0 "World" false) false false))))

(fn ConstructionScript)