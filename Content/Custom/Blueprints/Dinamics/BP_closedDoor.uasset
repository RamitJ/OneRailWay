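; BP_closedDoor is an interactable door that only opens once its power has been switched on.
; A box overlap shows or hides an interaction prompt widget.
; Interact either alternates a timeline that swings the mesh's yaw open and closed, or, without power, shows a find-the-power-switch widget for a few seconds.
; SwitchOn enables power and changes the plane's material.
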(event OnComponentBeginOverlap(Box)
  (params (OverlappedComponent :type Primitive%20Component%20Object%20Reference) (OtherActor :type Actor%20Object%20Reference) (OtherComp :type Primitive%20Component%20Object%20Reference) (OtherBodyIndex :type Integer) (bFromSweep :type Boolean) (SweepResult :type Hit%20Result%20Structure%20%28by%20ref%29))
  (bind _output_get (Variables|Default|SetESignWidget (Variables|Default|GetESignWidget)))
  (Widget|SetVisibility _output_get "Visible"))

(event OnComponentEndOverlap(Box)
  (params (OverlappedComponent :type Primitive%20Component%20Object%20Reference) (OtherActor :type Actor%20Object%20Reference) (OtherComp :type Primitive%20Component%20Object%20Reference) (OtherBodyIndex :type Integer))
  (bind _output_get (Variables|Default|SetESignWidget (Variables|Default|GetESignWidget)))
  (Widget|SetVisibility _output_get "Hidden"))

(event Custom|SwitchOn
  (Variables|Default|SetPowerOn true)
  (Rendering|Material|SetMaterial (Variables|Default|GetPlane) 0 "/Engine/BasicShapes/BasicShapeMaterial.BasicShapeMaterial"))

(event EventBeginPlay
  (bind _returnvalue (UserInterface|CreateWidget "/Game/Custom/Widgets/WB_ESign.WB_ESign_C"))
  (bind _output_get (Variables|Default|SetESignWidget _returnvalue))
  (UserInterface|Viewport|AddtoViewport _output_get 0)
  (Widget|SetVisibility _output_get "Hidden"))

(event EventInteract
  (if (Variables|Default|GetPowerOn)
    (Utilities|FlowControl|FlipFlop
      (:A
        (bind _newtrack_0 (Timeline|Timeline Play)
          (:Update
            (Transformation|SetRelativeRotation (Variables|Default|GetStaticMesh) (Math|Rotator|MakeRotator 0.0 0.0 (Math|Float|Lerp 9e+01 -35.0 _newtrack_0)) false false))))
      (:B
        (Timeline|Timeline Reverse)))
    (else
      (bind _returnvalue (UserInterface|CreateWidget "/Game/Custom/Widgets/WB_FindPowerSwitch.WB_FindPowerSwitch_C"))
      (bind _output_get (Variables|Default|SetNoPower _returnvalue))
      (UserInterface|Viewport|AddtoViewport _output_get 0)
      (Utilities|FlowControl|Delay 3.0)
      (Widget|RemovefromParent (Variables|Default|GetNoPower)))))

(fn ConstructionScript)