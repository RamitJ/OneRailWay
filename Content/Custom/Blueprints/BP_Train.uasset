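; BP_Train is a train actor with a toggleable sliding door, a repairable condition value and a spawned turret.
; Interact alternates playing and reversing a timeline that slides the door along its relative X axis.
; Condition starts below maximum, and each Repaired event raises it up to that cap.
; BeginPlay spawns the turret at an Arrow component after a short delay, while Tick prints Condition on screen for debugging.
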(event Custom|Repaired
  (bind _train (Variables|Default|GetTrain))
  (bind _output_get (Variables|BP_Train_C|SetCondition _train (Math|Integer|Clamp(Integer) (+ (Variables|BP_Train_C|GetCondition _train) 50) 0 (Variables|Default|GetMaxCondition))))
  (Development|PrintString (Utilities|String|ToString(Integer) _output_get) true true "(R=0.000000,G=1.000000,B=0.378531,A=1.000000)" 3.0))

(event EventTick
  (params (DeltaSeconds :type Float%20%28single-precision%29))
  (Development|PrintString (Utilities|String|ToString(Integer) (Variables|Default|GetCondition)) true true "(R=0.000000,G=0.660000,B=1.000000,A=1.000000)" DeltaSeconds))

(event EventBeginPlay
  (Variables|Default|SetCondition (- (Variables|Default|GetMaxCondition) 200))
  (Utilities|FlowControl|Delay 3.0)
  (Game|SpawnActorfromClass "/Game/Custom/Blueprints/TrainActors/Turret.Turret_C" (Transformation|GetWorldTransform (Variables|Default|GetArrow)) "Undefined" 0 0))

(event EventInteract
  (bind _door (Variables|Default|GetDoor))
  (bind _relativelocation (Variables|/Script/Engine.SceneComponent|GetRelativeLocation _door))
  (Utilities|FlowControl|FlipFlop
    (:A
      (bind _newtrack_0 (Timeline|SlideDoor Play)
        (:Update
          (Transformation|SetRelativeLocation _door (Math|Vector|MakeVector (Math|Float|Lerp 6e+02 7.7e+02 _newtrack_0) (.y _relativelocation) (.z _relativelocation)) false false))))
    (:B
      (Timeline|SlideDoor Reverse))))

(fn ConstructionScript)