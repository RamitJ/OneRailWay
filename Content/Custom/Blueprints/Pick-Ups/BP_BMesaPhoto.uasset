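; Pick-up actor for the Black Mesa photo item that the first-person player can collect.
; Overlapping its sphere creates and shows a new WB_ESign widget, and ending the overlap hides it.
; PickUpItem returns the BlackMesaPhoto item and triggers destroyitem, which sets HasBMphoto on the player character and destroys the actor after a short delay.
; Interact and LightOffPlaces are empty.
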(event OnComponentBeginOverlap(Sphere1)
  (params (OverlappedComponent :type Primitive%20Component%20Object%20Reference) (OtherActor :type Actor%20Object%20Reference) (OtherComp :type Primitive%20Component%20Object%20Reference) (OtherBodyIndex :type Integer) (bFromSweep :type Boolean) (SweepResult :type Hit%20Result%20Structure%20%28by%20ref%29))
  (bind _returnvalue (UserInterface|CreateWidget "/Game/Custom/Widgets/WB_ESign.WB_ESign_C"))
  (bind _output_get (Variables|Default|SetESignWidget _returnvalue))
  (UserInterface|Viewport|AddtoViewport _output_get 0)
  (Widget|SetVisibility _output_get "Visible"))

(event OnComponentEndOverlap(Sphere1)
  (params (OverlappedComponent :type Primitive%20Component%20Object%20Reference) (OtherActor :type Actor%20Object%20Reference) (OtherComp :type Primitive%20Component%20Object%20Reference) (OtherBodyIndex :type Integer))
  (bind _output_get (Variables|Default|SetESignWidget (Variables|Default|GetESignWidget)))
  (Widget|SetVisibility _output_get "Hidden"))

(event Custom|destroy%20item
  (bind _asbp_first_person_character (Utilities|Casting|CastToBP_FirstPersonCharacter (Game|GetPlayerCharacter 0)))
  (Variables|/Game/FirstPerson/Blueprints/BP_FirstPersonCharacter.BP_FirstPersonCharacter_C|SetHasBMphoto _asbp_first_person_character true)
  (Utilities|FlowControl|Delay 0.1)
  (Actor|DestroyActor))

(event Custom|LightOffPlaces)

(fn ConstructionScript)

(fn Interact
  (return))

(fn Pick-UpItem
  (Development|PrintString "item picked")
  (CallFunction|DestroyItem)
  (return (Variables|Default|GetBlack%20Mesa%20photo)))