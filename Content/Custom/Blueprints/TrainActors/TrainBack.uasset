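; TrainBack is a train actor Blueprint that shows a train condition bar on screen while something overlaps its Box.
; On BeginPlay it creates a WB_TrainConditionBar widget, stores it, adds it to the viewport and hides it.
; The Box's begin and end overlap events toggle that widget between visible and hidden, with no check on which actor triggers them.
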(event OnComponentBeginOverlap(Box)
  (params (OverlappedComponent :type Primitive%20Component%20Object%20Reference) (OtherActor :type Actor%20Object%20Reference) (OtherComp :type Primitive%20Component%20Object%20Reference) (OtherBodyIndex :type Integer) (bFromSweep :type Boolean) (SweepResult :type Hit%20Result%20Structure%20%28by%20ref%29))
  ;[1 1 1] Condition widget
  (bind _output_get (Variables|Default|SetConditionWidget (Variables|Default|GetConditionWidget)))
  (Widget|SetVisibility _output_get "Visible"))

(event OnComponentEndOverlap(Box)
  (params (OverlappedComponent :type Primitive%20Component%20Object%20Reference) (OtherActor :type Actor%20Object%20Reference) (OtherComp :type Primitive%20Component%20Object%20Reference) (OtherBodyIndex :type Integer))
  ;[1 1 1] Condition widget
  (bind _output_get (Variables|Default|SetConditionWidget (Variables|Default|GetConditionWidget)))
  (Widget|SetVisibility _output_get "Hidden"))

(event EventBeginPlay
  ;[1 1 1] Condition widget
  (bind _returnvalue (UserInterface|CreateWidget "/Game/Custom/Widgets/WB_TrainConditionBar.WB_TrainConditionBar_C"))
  (bind _output_get (Variables|Default|SetConditionWidget _returnvalue))
  (UserInterface|Viewport|AddtoViewport _output_get 0)
  (Widget|SetVisibility _output_get "Hidden"))

(fn ConstructionScript)