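; Heater actor for the train actors set that applies damage to whatever actor is inside its sphere.
; Sphere begin overlap stores any overlapping actor as Player and adds a new Frostbyte widget to the viewport.
; Tick applies the Damage value to Player every frame, without delta-time scaling.
; End overlap clears Player but leaves the widget on screen.
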(event OnComponentBeginOverlap(Sphere)
  (params (OverlappedComponent :type Primitive%20Component%20Object%20Reference) (OtherActor :type Actor%20Object%20Reference) (OtherComp :type Primitive%20Component%20Object%20Reference) (OtherBodyIndex :type Integer) (bFromSweep :type Boolean) (SweepResult :type Hit%20Result%20Structure%20%28by%20ref%29))
  (Variables|Default|Setplayer OtherActor)
  (bind _returnvalue (UserInterface|CreateWidget "/Game/Custom/Widgets/WB_Frostbyte.WB_Frostbyte_C"))
  (bind _output_get (Variables|Default|Setfrostbite%20wb _returnvalue))
  (UserInterface|Viewport|AddtoViewport _output_get 0)
  (Widget|SetVisibility _output_get "Visible"))

(event OnComponentEndOverlap(Sphere)
  (params (OverlappedComponent :type Primitive%20Component%20Object%20Reference) (OtherActor :type Actor%20Object%20Reference) (OtherComp :type Primitive%20Component%20Object%20Reference) (OtherBodyIndex :type Integer))
  (Variables|Default|Setplayer 0))

(event EventBeginPlay)

(event Collision|EventActorBeginOverlap
  (params (OtherActor :type Actor%20Object%20Reference)))

(event EventTick
  (params (DeltaSeconds :type Float%20%28single-precision%29))
  (Game|Damage|ApplyDamage (Variables|Default|Getplayer) (Variables|Default|Getdamage) 0 0))

(fn ConstructionScript)