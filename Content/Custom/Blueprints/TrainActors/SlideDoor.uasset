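; SlideDoor is a train actor that shows an on-screen WB_ESign widget, likely an interact prompt, while something overlaps its Box.
; BeginPlay creates the widget, adds it to the viewport and hides it.
; Box begin and end overlap events toggle its visibility without checking which actor overlapped.
; The graphs contain no door movement or input handling, and the construction script is empty.
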(event OnComponentBeginOverlap(Box)
  (params (OverlappedComponent :type Primitive%20Component%20Object%20Reference) (OtherActor :type Actor%20Object%20Reference) (OtherComp :type Primitive%20Component%20Object%20Reference) (OtherBodyIndex :type Integer) (bFromSweep :type Boolean) (SweepResult :type Hit%20Result%20Structure%20%28by%20ref%29))
  (bind _output_get (Variables|Default|SetESignWidget (Variables|Default|GetESignWidget)))
  (Widget|SetVisibility _output_get "Visible"))

(event OnComponentEndOverlap(Box)
  (params (OverlappedComponent :type Primitive%20Component%20Object%20Reference) (OtherActor :type Actor%20Object%20Reference) (OtherComp :type Primitive%20Component%20Object%20Reference) (OtherBodyIndex :type Integer))
  (bind _output_get (Variables|Default|SetESignWidget (Variables|Default|GetESignWidget)))
  (Widget|SetVisibility _output_get "Hidden"))

(event EventBeginPlay
  (bind _returnvalue (UserInterface|CreateWidget "/Game/Custom/Widgets/WB_ESign.WB_ESign_C"))
  (bind _output_get (Variables|Default|SetESignWidget _returnvalue))
  (UserInterface|Viewport|AddtoViewport _output_get 0)
  (Widget|SetVisibility _output_get "Hidden"))

(fn ConstructionScript)