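; FlipDoor is an interactable door actor that flips open and closed and shows an on-screen prompt widget nearby.
; It creates a hidden WB_ESign widget on BeginPlay, and Box overlap events show and hide it.
; The Interact event uses a FlipFlop to play or reverse a Timeline, which lerps the Cube's relative roll and height.
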(event OnComponentBeginOverlap(Box)
  (params (OverlappedComponent :type Primitive%20Component%20Object%20Reference) (OtherActor :type Actor%20Object%20Reference) (OtherComp :type Primitive%20Component%20Object%20Reference) (OtherBodyIndex :type Integer) (bFromSweep :type Boolean) (SweepResult :type Hit%20Result%20Structure%20%28by%20ref%29))
  (bind _output_get (Variables|Default|SetESignWidget (Variables|Default|GetESignWidget)))
  (Widget|SetVisibility _output_get "Visible"))

(event OnComponentEndOverlap(Box)
  (params (OverlappedComponent :type Primitive%20Component%20Object%20Reference) (OtherActor :type Actor%20Object%20Reference) (OtherComp :type Primitive%20Component%20Object%20Reference) (OtherBodyIndex :type Integer))
  (bind _output_get (Variables|Default|SetESignWidget (Variables|Default|GetESignWidget)))
  (Widget|SetVisibility _output_get "Hidden"))

(event EventBeginPlay
  (bind _returnvalue (UserInterface|CreateWidget "/Game/Custom/Widgets/WB_ESign.WB_ESign_C"))
  (bind _output_get (Variables|Default|SetESignWidget _returnvalue))
  (UserInterface|Viewport|AddtoViewport _output_get 0)
  (Widget|SetVisibility _output_get "Hidden"))

(event EventInteract
  (Utilities|FlowControl|FlipFlop
    (:A
      (bind _newtrack_0 (Timeline|Timeline Play)
        (:Update
          (Transformation|SetRelativeRotation (Variables|Default|GetCube) (Math|Rotator|MakeRotator (Math|Float|Lerp 0.0 -9e+01 _newtrack_0) 0.0 0.0) false false)
          (Transformation|SetRelativeLocation (Variables|Default|GetCube) (Math|Vector|MakeVector 0.0 0.0 (Math|Float|Lerp 1e+02 1.5e+02 _newtrack_0)) false false))))
    (:B
      (Timeline|Timeline Reverse))))

(fn ConstructionScript)