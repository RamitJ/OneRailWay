(event Custom|BuildTurret
  ;[1 1 1] Building
  (Utilities|FlowControl|Delay 3.0)
  (bind _returnvalue (Game|SpawnActorfromClass "/Game/Custom/Blueprints/TrainActors/Turret.Turret_C" (Transformation|GetWorldTransform (Variables|Default|GetPlaceTurret)) "Undefined" 0 0))
  (Transformation|AttachComponentToComponent _returnvalue (Variables|Default|GetDefaultSceneRoot) "None" "KeepWorld" "KeepWorld" "KeepWorld" true)
  (Variables|Default|Set1stLvlTurret true))

(event Custom|ConnectFirstWagon
  (Components|Timeline|SetPlayRate (Variables|Default|GetMove%20Train) (/ 1.0 (Variables|Default|GetTime%20to%20Comlete%20Route)))
  (bind _newtrack_1 (Timeline|Move%20Train Play)
    (:Update
      (Transformation|SetActorTransform (Math|Transform|MakeTransform (Spline|GetLocationatDistanceAlongSpline (Variables|/Game/Custom/RailWay/BP_1stWagonRouteToTrain.BP_1stWagonRouteToTrain_C|GetSpline (Variables|Default|GetSplineRef)) (Math|Float|Lerp 0.0 (Spline|GetSplineLength (Variables|/Game/Custom/RailWay/BP_1stWagonRouteToTrain.BP_1stWagonRouteToTrain_C|GetSpline (Variables|Default|GetSplineRef))) _newtrack_1) "World") "5.000000,17.000000,0.000000" "1.000000,1.000000,1.000000")))))

(event Custom|BuildLocator
  ;[1 1 1] Building
  (Utilities|FlowControl|Delay 3.0)
  (bind _returnvalue (Game|SpawnActorfromClass "/Game/Custom/Blueprints/TrainActors/Locator.Locator_C" (Transformation|GetWorldTransform (Variables|Default|GetPlaceLocator)) "Undefined" 0 0))
  (Transformation|AttachComponentToComponent _returnvalue (Variables|Default|GetDefaultSceneRoot) "None" "KeepWorld" "KeepWorld" "KeepWorld" true)
  (Variables|Default|Set1stLvlLocator true))

(event Custom|BuildHeater
  ;[1 1 1] Building
  (Utilities|FlowControl|Delay 3.0)
  (bind _returnvalue (Game|SpawnActorfromClass "/Game/Custom/Blueprints/TrainActors/Heater.Heater_C" (Transformation|GetWorldTransform (Variables|Default|GetPlaceHeater)) "Undefined" 0 0))
  (Transformation|AttachComponentToComponent _returnvalue (Variables|Default|GetDefaultSceneRoot) "None" "KeepWorld" "KeepWorld" "KeepWorld" true)
  (Variables|Default|Set1stLvlHeater true))

(event Custom|LightsOn
  ;[1 1 1] Highlight build places
  (Utilities|FlowControl|Sequence
    (:then_0
      (Rendering|Components|Light|SetIntensity (Variables|Default|GetPointLight1) 2e+03))))

(event Custom|LightsOff
  ;[1 1 1] Highlight build places
  (Utilities|FlowControl|Sequence
    (:then_0
      (Rendering|Components|Light|SetIntensity (Variables|Default|GetPointLight1) 0.0))))

(event Custom|PutBMPhoto
  (bind _returnvalue (Game|SpawnActorfromClass "/Game/Custom/Blueprints/Pick-Ups/BP_BMesaPhoto.BP_BMesaPhoto_C" (Transformation|GetWorldTransform (Variables|Default|GetPlaceBMPhoto)) "Undefined" 0 0))
  (Transformation|AttachComponentToComponent _returnvalue (Variables|Default|GetDefaultSceneRoot) "None" "KeepWorld" "KeepWorld" "KeepWorld" true)
  (bind _returnvalue_2 (Actor|GetActorOfClass "/Game/Custom/Blueprints/Pick-Ups/BP_BMesaPhoto.BP_BMesaPhoto_C"))
  (Collision|SetCollisionEnabled (Variables|/Game/Custom/Blueprints/Pick-Ups/BP_BMesaPhoto.BP_BMesaPhoto_C|GetSphere1 _returnvalue_2) "NoCollision"))

(event Custom|LaunchWagon
  (bind _1stslinerouteref (Variables|Default|Get1stSlineRouteRef))
  (bind _spline (Variables|/Game/Custom/RailWay/BP_RailWayRoute.BP_RailWayRoute_C|GetSpline _1stslinerouteref))
  (if true
    (Components|Timeline|SetPlayRate (Variables|Default|GetMove%20Train1) (/ 1.0 (Variables|Default|GetTime%20To%20Complete%20Route%202)))
    (bind _newtrack_0 (Timeline|Move%20Train1 Play)
      (:Update
        (Transformation|SetActorTransform (Math|Transform|MakeTransform (Spline|GetLocationatDistanceAlongSpline _spline (Math|Float|Lerp 0.0 (Spline|GetSplineLength (Variables|/Game/Custom/RailWay/BP_RailWayRoute.BP_RailWayRoute_C|GetSpline (Variables|Default|Get1stSlineRouteRef))) _newtrack_0) "World") (Spline|GetRotationatDistanceAlongSpline _spline (Math|Float|Lerp 0.0 (Spline|GetSplineLength (Variables|/Game/Custom/RailWay/BP_RailWayRoute.BP_RailWayRoute_C|GetSpline (Variables|Default|Get1stSlineRouteRef))) _newtrack_0) "World") "1.000000,1.000000,1.000000"))))))

(event EventBeginPlay
  (Utilities|FlowControl|Sequence
    (:then_0
      (bind _returnvalue (Actor|GetActorOfClass "/Game/Custom/RailWay/BP_1stWagonRouteToTrain.BP_1stWagonRouteToTrain_C"))
      (Variables|Default|SetSplineRef _returnvalue))
    (:then_1
      (bind _returnvalue_2 (Actor|GetActorOfClass "/Game/Custom/RailWay/BP_WagonRailWayRoute.BP_WagonRailWayRoute_C"))
      (Variables|Default|Set1stWagonSplineRouteRef _returnvalue_2))
    (:then_2
      (bind _returnvalue_3 (Actor|GetActorOfClass "/Game/Custom/RailWay/BP_RailWayRoute.BP_RailWayRoute_C"))
      (Variables|Default|Set1stSlineRouteRef _returnvalue_3))
    (:then_3
      (bind _returnvalue_4 (Actor|GetActorOfClass "/Game/Custom/RailWay/BP_2ndRailWayRoute.BP_2ndRailWayRoute_C"))
      (Variables|Default|Set2ndSplineRouteRef _returnvalue_4))))

(event EventInteract
  (bind _door (Variables|Default|GetDoor))
  (bind _relativelocation (Variables|/Script/Engine.SceneComponent|GetRelativeLocation _door))
  (Utilities|FlowControl|FlipFlop
    (:A
      (bind _newtrack_0 (Timeline|SlideDoor Play)
        (:Update
          (Transformation|SetRelativeLocation _door (Math|Vector|MakeVector (Math|Float|Lerp 6e+02 7.7e+02 _newtrack_0) (.y _relativelocation) (.z _relativelocation)) false false))))
    (:B
      (Timeline|SlideDoor Reverse))))

(fn ConstructionScript)