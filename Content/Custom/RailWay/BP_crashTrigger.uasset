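; BP_crashTrigger is a railway trigger that crashes the drop bridge and switches the train's route.
; When something overlaps its Box while WagonSent is true, it plays a world camera shake at its own location.
; After a short delay it finds Drop_bridge by class and calls Crash, then finds BP_Train and flips its route flags from first to second.
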(event OnComponentBeginOverlap(Box)
  (params (OverlappedComponent :type Primitive%20Component%20Object%20Reference) (OtherActor :type Actor%20Object%20Reference) (OtherComp :type Primitive%20Component%20Object%20Reference) (OtherBodyIndex :type Integer) (bFromSweep :type Boolean) (SweepResult :type Hit%20Result%20Structure%20%28by%20ref%29))
  (if (Variables|Default|Getwagon%20sent)
    (Camera|PlayWorldCameraShake "/Game/Custom/CameraShakes/BP_HangarDoorCameraShake.BP_HangarDoorCameraShake_C" (Transformation|GetActorLocation) 0.0 3e+02)
    (Utilities|FlowControl|Delay 2.0)
    (Utilities|FlowControl|Sequence
      (:then_0
        (bind _returnvalue (Actor|GetActorOfClass "/Game/Custom/RailWay/drop_bridge.drop_bridge_C"))
        (Default|Crash _returnvalue))
      (:then_1
        (bind _returnvalue_2 (Actor|GetActorOfClass "/Game/Custom/Blueprints/BP_Train.BP_Train_C"))
        (Variables|/Game/Custom/Blueprints/BP_Train.BP_Train_C|Set1stRoute _returnvalue_2 false)
        (Variables|/Game/Custom/Blueprints/BP_Train.BP_Train_C|Set2ndRoute _returnvalue_2 true)))))

(event EventBeginPlay)

(event Collision|EventActorBeginOverlap
  (params (OtherActor :type Actor%20Object%20Reference)))

(event EventTick
  (params (DeltaSeconds :type Float%20%28single-precision%29)))

(fn ConstructionScript)